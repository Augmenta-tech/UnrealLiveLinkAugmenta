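; Augmenta visualizer actor that mirrors tracked objects, scene and video output as attached child actors.
; It binds to AugmentaEventDispatcher events to spawn, transform or destroy these actors, keeping objects in a map keyed by Id.
; A looping timer removes objects whose last update is too old, covering missed leave messages.
; Disabling visualization stops spawning and updates and hides the scene and video output actors; source destruction destroys all spawned actors.
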(event Custom|OnAugmentaObjectUpdated_Event
  (params (AugmentaObject :type Live%20Link%20Augmenta%20Object%20Structure))
  ;[1 1 1] Bind to OnAugmentaObjectUpdated
  (Augmenta|OnObjectUpdatedReceived AugmentaObject))

(event Custom|OnAugmentaObjectLeft_Event
  (params (AugmentaObject :type Live%20Link%20Augmenta%20Object%20Structure))
  ;[1 1 1] Bind to OnAugmentaObjectLeft
  (Augmenta|OnObjectLeftReceived AugmentaObject))

(event Custom|OnAugmentaSceneUpdated_Event
  (params (AugmentaScene :type Live%20Link%20Augmenta%20Scene%20Structure))
  ;[1 1 1] Bind to OnAugmentaSceneUpdated
  (Augmenta|UpdateAugmentaScene AugmentaScene))

(event Custom|OnAugmentaVideoOutputUpdated_Event
  (params (AugmentaVideoOutput :type Live%20Link%20Augmenta%20Video%20Output%20Structure))
  ;[1 1 1] Bind to OnAugmentaVideoOutputUpdated
  (Augmenta|UpdateAugmentaVideoOutput AugmentaVideoOutput))

(event Custom|OnAugmentaSourceDestroyed_Event
  ;[1 1 1] Bind to OnAugmentaSourceDestroyed
  (Augmenta|OnSourceDestroyed))

(event Custom|OnCleanupTimerElapsed_Event
  ;[1 1 1] Start the cleanup inactive actors loop. This is to ensure no actors remains forever if their leaving message was missed.
  (Augmenta|CleanUpInactiveActors))

(event EventBeginPlay
  (Utilities|IsValid (Variables|Augmenta|GetAugmentaEventDispatcher)
    (:Is%20Valid
      (Utilities|FlowControl|Sequence
        (:then_0
          (if (Variables|Augmenta|GetbDisableAtStart)
            (Augmenta|DisableVisualization)))
        (:then_1
          ;[1 1 1] Bind to OnAugmentaObjectUpdated
          (EventDispatchers|BindEventtoOnAugmentaObjectUpdated (Variables|Augmenta|GetAugmentaEventDispatcher) (delegate Custom|OnAugmentaObjectUpdated_Event))
          ;[1 1 1] Bind to OnAugmentaObjectLeft
          (EventDispatchers|BindEventtoOnAugmentaObjectLeft (Variables|Augmenta|GetAugmentaEventDispatcher) (delegate Custom|OnAugmentaObjectLeft_Event))
          ;[1 1 1] Bind to OnAugmentaSceneUpdated
          (EventDispatchers|BindEventtoOnAugmentaSceneUpdated (Variables|Augmenta|GetAugmentaEventDispatcher) (delegate Custom|OnAugmentaSceneUpdated_Event))
          ;[1 1 1] Bind to OnAugmentaVideoOutputUpdated
          (EventDispatchers|BindEventtoOnAugmentaVideoOutputUpdated (Variables|Augmenta|GetAugmentaEventDispatcher) (delegate Custom|OnAugmentaVideoOutputUpdated_Event))
          ;[1 1 1] Bind to OnAugmentaSourceDestroyed
          (EventDispatchers|BindEventtoOnAugmentaSourceDestroyed (Variables|Augmenta|GetAugmentaEventDispatcher) (delegate Custom|OnAugmentaSourceDestroyed_Event)))
        (:then_2
          ;[1 1 1] Start the cleanup inactive actors loop. This is to ensure no actors remains forever if their leaving message was missed.
          (Utilities|Time|SetTimerbyEvent (delegate Custom|OnCleanupTimerElapsed_Event) (Variables|Augmenta|GetActorsCleanUpRate) true))))
    (:Is%20Not%20Valid
      (Development|PrintString "Augmenta Event Dispatcher not valid in Augmenta Visualizer." true true "(R=1.000000,G=0.000000,B=0.000000,A=1.000000)"))))

(fn ConstructionScript)

(fn OnObjectUpdatedReceived
  (params (AugmentaObject :type Live%20Link%20Augmenta%20Object%20Structure))
  ;[1 1 1] Check if a spawned actor already has this Id
  (if (Variables|Augmenta|GetbVisualizationEnabled)
    (if (Utilities|Map|Contains (Variables|Augmenta|GetAugmentaObjectActors) (.Id (Utilities|Struct|BreakLiveLinkAugmentaObject AugmentaObject)))
      (Augmenta|UpdateSpawnedActor AugmentaObject)
      (else
        (Augmenta|SpawnActor AugmentaObject)))))

(fn OnObjectLeftReceived
  (params (AugmentaObject :type Live%20Link%20Augmenta%20Object%20Structure))
  (bind _id (Utilities|Struct|BreakLiveLinkAugmentaObject AugmentaObject))
  (bind _augmentaobjectactors (Variables|Augmenta|GetAugmentaObjectActors))
  (bind (_value _returnvalue) (Utilities|Map|Find _augmentaobjectactors _id))
  ;[1 1 1] Check if a spawned actor already has this Id
  (if _returnvalue
    ;[1 1 1] If a spawned actor exists with this Id, destroy it and remove it from the InstantiatedActors.
    (Actor|DestroyActor _value)
    (Utilities|Map|Remove (Variables|Augmenta|GetAugmentaObjectActors) _id)))

(fn UpdateSpawnedActor
  (params (AugmentaObject :type Live%20Link%20Augmenta%20Object%20Structure))
  (bind (_frame _id _oid _age _centroid _velocity _orientation _boundingrectpos _boundingrectsize _boundingrectrotation _height _highest _distance _reflectivity _lastupdatetime _position _rotation _scale) (Utilities|Struct|BreakLiveLinkAugmentaObject AugmentaObject))
  (bind _augmentaobjectactors (Variables|Augmenta|GetAugmentaObjectActors))
  (bind _value (Utilities|Map|Find _augmentaobjectactors _id))
  ;[1 1 1] Update actor location, rotation and scale
  (Transformation|SetActorRelativeLocation _value _position)
  (Transformation|SetActorRelativeRotation _value (Class|KismetMathLibrary|QuatRotator _rotation))
  (Transformation|SetActorRelativeScale3D _value _scale)
  ;[1 1 1] Update the LastUpdateTime of the Actor
  (Variables|/LiveLinkAugmenta/Blueprints/BP_AugmentaObject.BP_AugmentaObject_C|SetLastUpdateTime _value (Utilities|Time|GetGameTimeinSeconds)))

(fn SpawnActor
  (params (AugmentaObject :type Live%20Link%20Augmenta%20Object%20Structure))
  (bind (_frame _id _oid _age _centroid _velocity _orientation _boundingrectpos _boundingrectsize _boundingrectrotation _height _highest _distance _reflectivity _lastupdatetime _position _rotation _scale) (Utilities|Struct|BreakLiveLinkAugmentaObject AugmentaObject))
  (bind _augmentaobjectactorclass (Variables|Augmenta|GetAugmentaObjectActorClass))
  ;[1 1 1] Spawn new actor and add it to the Spawned Actors
  (if (Utilities|IsValidClass _augmentaobjectactorclass)
    (bind _returnvalue (Game|SpawnActorfromClass _augmentaobjectactorclass (Math|Transform|MakeTransform _position (Class|KismetMathLibrary|QuatRotator _rotation) _scale) "Undefined" "SelectDefaultAtRuntime" self 0))
    (Utilities|Map|Add (Variables|Augmenta|GetAugmentaObjectActors) _id (.AsBP%20Augmenta%20Object (Utilities|Casting|CastToBP_AugmentaObject _returnvalue)))
    (Transformation|AttachActorToActor _returnvalue self "None" "KeepRelative" "KeepRelative" "KeepRelative" true)))

(fn UpdateAugmentaScene
  (params (AugmentaScene :type Live%20Link%20Augmenta%20Scene%20Structure))
  (bind _scale (Utilities|Struct|BreakLiveLinkAugmentaScene AugmentaScene))
  (bind _augmentasceneactorclass (Variables|Augmenta|GetAugmentaSceneActorClass))
  (if (Variables|Augmenta|GetbVisualizationEnabled)
    (Utilities|IsValid (Variables|Augmenta|GetAugmentaSceneActor)
      (:Is%20Valid
        ;[1 1 1] Update scene size
        (Transformation|SetActorRelativeScale3D (Variables|Augmenta|GetAugmentaSceneActor) _scale))
      (:Is%20Not%20Valid
        ;[1 1 1] Instantiate Augmenta scene actor
        (if (Utilities|IsValidClass _augmentasceneactorclass)
          (bind _returnvalue (Game|SpawnActorfromClass _augmentasceneactorclass (Math|Transform|MakeTransform "0, 0, 0" "0, 0, 0" _scale) "Undefined" "SelectDefaultAtRuntime" self 0))
          (bind _output_get (Variables|Augmenta|SetAugmentaSceneActor _returnvalue))
          (Transformation|AttachActorToActor _output_get self "None" "KeepRelative" "KeepRelative" "KeepRelative" true))))))

(fn UpdateAugmentaVideoOutput
  (params (AugmentaVideoOutput :type Live%20Link%20Augmenta%20Video%20Output%20Structure))
  (bind (_offset _size _resolution _position _rotation _scale) (Utilities|Struct|BreakLiveLinkAugmentaVideoOutput AugmentaVideoOutput))
  (bind _augmentavideooutputactorclass (Variables|Augmenta|GetAugmentaVideoOutputActorClass))
  (if (Variables|Augmenta|GetbVisualizationEnabled)
    (Utilities|IsValid (Variables|Augmenta|GetAugmentaVideoOutputActor)
      (:Is%20Valid
        ;[1 1 1] Update video output scale and location
        (Transformation|SetActorRelativeScale3D (Variables|Augmenta|GetAugmentaVideoOutputActor) _scale)
        (Transformation|SetActorRelativeLocation (Variables|Augmenta|GetAugmentaVideoOutputActor) _position false true))
      (:Is%20Not%20Valid
        ;[1 1 1] Instantiate Augmenta video output actor
        (if (Utilities|IsValidClass _augmentavideooutputactorclass)
          (bind _returnvalue (Game|SpawnActorfromClass _augmentavideooutputactorclass (Math|Transform|MakeTransform _position (Class|KismetMathLibrary|QuatRotator _rotation) _scale) "Undefined" "SelectDefaultAtRuntime" self 0))
          (bind _output_get (Variables|Augmenta|SetAugmentaVideoOutputActor _returnvalue))
          (Transformation|AttachActorToActor _output_get self "None" "KeepRelative" "KeepRelative" "KeepRelative" true))))))

(fn OnSourceDestroyed
  (bind _augmentasceneactor (Variables|Augmenta|GetAugmentaSceneActor))
  (bind _augmentavideooutputactor (Variables|Augmenta|GetAugmentaVideoOutputActor))
  (Utilities|FlowControl|Sequence
    (:then_0
      ;[1 1 1] Destroy scene actor
      (Utilities|IsValid _augmentasceneactor
        (:Is%20Valid
          (Actor|DestroyActor _augmentasceneactor))))
    (:then_1
      ;[1 1 1] Destroy video output actor
      (Utilities|IsValid _augmentavideooutputactor
        (:Is%20Valid
          (Actor|DestroyActor _augmentavideooutputactor))))
    (:then_2
      ;[1 1 1] Destroy all object actors and clear the object actors map
      (bind _keys (Utilities|Map|Keys (Variables|Augmenta|GetAugmentaObjectActors)))
      (for _array_element _keys
        (Utilities|IsValid (.Value (Utilities|Map|Find (Variables|Augmenta|GetAugmentaObjectActors) _array_element))
          (:Is%20Valid
            (Actor|DestroyActor (.Value (Utilities|Map|Find (Variables|Augmenta|GetAugmentaObjectActors) _array_element))))))
      (Utilities|Map|Clear (Variables|Augmenta|GetAugmentaObjectActors)))))

(fn CleanUpInactiveActors
  (bind _keys (Utilities|Map|Keys (Variables|Augmenta|GetAugmentaObjectActors)))
  (for _array_element _keys
    (if (> (- (Utilities|Time|GetGameTimeinSeconds) (Variables|/LiveLinkAugmenta/Blueprints/BP_AugmentaObject.BP_AugmentaObject_C|GetLastUpdateTime (.Value (Utilities|Map|Find (Variables|Augmenta|GetAugmentaObjectActors) _array_element)))) (Variables|Augmenta|GetActorsMaxInactiveTime))
      ;[1 1 1] Destroy the actor and remove it from the map
      (Actor|DestroyActor (.Value (Utilities|Map|Find (Variables|Augmenta|GetAugmentaObjectActors) _array_element)))
      (Utilities|Map|Remove (Variables|Augmenta|GetAugmentaObjectActors) _array_element))))

(fn EnableVisualization
  (Augmenta|SetVisualization true))

(fn DisableVisualization
  (Augmenta|SetVisualization false))

(fn SetVisualization
  (params (bEnabled :type Boolean))
  (bind _augmentasceneactor (Variables|Augmenta|GetAugmentaSceneActor))
  (bind _augmentavideooutputactor (Variables|Augmenta|GetAugmentaVideoOutputActor))
  (Variables|Augmenta|SetbVisualizationEnabled bEnabled)
  (Utilities|FlowControl|Sequence
    (:then_0
      ;[1 1 1] Update scene actor
      (Utilities|IsValid _augmentasceneactor
        (:Is%20Valid
          (Rendering|SetActorHiddenInGame _augmentasceneactor (not (Variables|Augmenta|GetbVisualizationEnabled))))))
    (:then_1
      ;[1 1 1] Update Video output actor visibility
      (Utilities|IsValid _augmentavideooutputactor
        (:Is%20Valid
          (Rendering|SetActorHiddenInGame _augmentavideooutputactor (not (Variables|Augmenta|GetbVisualizationEnabled))))))))